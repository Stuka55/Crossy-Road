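; Test chicken player Character for a hop-across-the-road game, with deaths by car and water.
; Axis input launches hops gated by a 0.6-second cooldown with a cluck, while timelines turn the mesh toward the hop.
; Death events squash or sink the chicken, show the game-over HUD and block movement.
; BeginPlay starts audio and the HUD, whose Chicken reference is unset; eagle-death functions are empty stubs.
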(event `FallInWater`
  (`self.K2_AddActorWorldOffset` (0.0 0.0 -500.0) false true)
  (bind _returnvalue (`|CreateWidget` "/Game/Blueprint/GameOverHUD.GameOverHUD_C" :!label _label))
  (`UserWidget.AddToViewport` _returnvalue 0)
  (set `PlayerController.bShowMouseCursor` true (`GameplayStatics.GetPlayerController` 0))
  (set `self.NotDead` false))

(event `HitSideOfCar`
  (`SceneComponent.SetWorldScale3D` (`self.StaticMesh`) (1.0 0.1 1.0))
  (goto _label))

(event `RanOverByCar`
  (`SceneComponent.SetWorldScale3D` (`self.StaticMesh`) (1.0 1.0 0.1))
  (goto _label))

(event `self.ReceiveTick`
  (params (DeltaSeconds :type "Float (single-precision)")))

(event `self.ReceiveBeginPlay`
  (`GameplayStatics.PlaySound2D` "/Game/audio/Rooster-morning-call.Rooster-morning-call" 1.0 1.0 0.0 null null)
  (`GameplayStatics.PlaySound2D` "/Game/audio/The-Good-the-Bad-and-the-Ugly.The-Good-the-Bad-and-the-Ugly" 1.0 1.0 0.0 null null)
  (bind _returnvalue (`|CreateWidget` "/Game/Blueprint/WBP_HUD.WBP_HUD_C"))
  (`UserWidget.AddToViewport` _returnvalue 0)
  (set `/Game/Blueprint/WBP_HUD.Chicken` null _returnvalue) ; I think this needs modifying in the hud section since this is a \ndifferent "chicken" (different class)\n\nif youre just copying nodes over then you can ignore this message
  (bind _output_get (set `self.MyHUD` _returnvalue))
  (`/Game/Blueprint/WBP_HUD.UpdateTapCounter` _output_get)
  (`/Game/Blueprint/WBP_HUD.UpdateCoinCounter` _output_get))

(event `InputAxis|JumpForward`
  (params (AxisValue :type "Float (single-precision)"))
  (bind _staticmesh (`self.StaticMesh`))
  (bind _staticmesh_2 (`self.StaticMesh`))
  (if (and (and (> (`KismetMathLibrary.Abs` AxisValue) 0.3) (`self.canmove`)) (`self.NotDead`))
    (`self.movementCooldown`)
    (`self.LaunchCharacter` (`KismetMathLibrary.MakeVector` (* AxisValue (`self.MovementSpace`)) 0.0 310.0) true true)
    (if (> AxisValue 0.3)
      (bind (_direction _newtrack_0) (`Timeline|Timeline_2` :!via `PlayFromStart`)
        (:`Update`
          (`SceneComponent.K2_SetWorldRotation` _staticmesh (`KismetMathLibrary.RLerp` (`SceneComponent.K2_GetComponentRotation` _staticmesh) (struct :`Yaw` 270.0) _newtrack_0 true) false false)))
      (else
        (bind (_direction_2 _newtrack_0_2) (`Timeline|Timeline_3` :!via `PlayFromStart`)
          (:`Update`
            (`SceneComponent.K2_SetWorldRotation` _staticmesh_2 (`KismetMathLibrary.RLerp` (`SceneComponent.K2_GetComponentRotation` _staticmesh_2) (struct :`Yaw` 90.0) _newtrack_0_2 true) false false)))))))

(event `InputAxis|JumpRight`
  (params (AxisValue :type "Float (single-precision)"))
  (bind _staticmesh (`self.StaticMesh`))
  (bind _staticmesh_2 (`self.StaticMesh`))
  (if (and (and (> (`KismetMathLibrary.Abs` AxisValue) 0.3) (`self.canmove`)) (`self.NotDead`))
    (`self.movementCooldown`)
    (`self.LaunchCharacter` (`KismetMathLibrary.MakeVector` 0.0 (* AxisValue (`self.MovementSpace`)) 150.0) true true)
    (if (> AxisValue 0.3)
      (bind (_direction _newtrack_0) (`Timeline|Timeline_0` :!via `PlayFromStart`)
        (:`Update`
          (`SceneComponent.K2_SetWorldRotation` _staticmesh_2 (`KismetMathLibrary.RLerp` (`SceneComponent.K2_GetComponentRotation` _staticmesh_2) (struct) _newtrack_0 true) false false)))
      (else
        (bind (_direction_2 _newtrack_0_2) (`Timeline|Timeline_1` :!via `PlayFromStart`)
          (:`Update`
            (`SceneComponent.K2_SetWorldRotation` _staticmesh (`KismetMathLibrary.RLerp` (`SceneComponent.K2_GetComponentRotation` _staticmesh) (struct :`Yaw` 180.0) _newtrack_0_2 true) false false)))))))

(event `movementCooldown`
  (`/Engine/EditorBlueprintResources/StandardMacros.DoOnce` false :!label _label_2
    (:`Completed`
      (`GameplayStatics.PlaySoundAtLocation` "/Game/audio/chickBawk1.chickBawk1" (`self.K2_GetActorLocation`) (struct) 1.0 1.0 0.0 null null null null)
      (set `self.canmove` false)
      (`KismetSystemLibrary.Delay` 0.6)
      (set `self.canmove` true)
      (goto _label_2 :!via `Reset`))))

(fn `ChickenDies`)

(fn `EagleKillChicken`)

(fn `UserConstructionScript`)