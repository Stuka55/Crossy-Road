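; BP_Lane is a lane actor with three mesh pieces for a chicken lane-crossing game.
; When BP_Chicken overlaps its trigger zone, it asks MyLaneSpawner to spawn another lane.
; RandomizeLane gives a first lane field meshes; otherwise it picks field, river, road or train track.
; A separate random roll and the FieldType1 flag can substitute the second field mesh, intended to alternate field colors.
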(event `self.TriggerZone.OnComponentBeginOverlap`
  (params (OverlappedComponent :type "PrimitiveComponent Object Reference") (OtherActor :type "Actor Object Reference") (OtherComp :type "PrimitiveComponent Object Reference") (OtherBodyIndex :type Integer) (bFromSweep :type Boolean) (SweepResult :type "HitResult Structure (by ref)"))
  (cast `/Game/Blueprint/BP_Chicken` OtherActor)
  (`/Game/Blueprint/BP_LaneSpawner.SpawnLaneAtSpawnPoint` (`self.MyLaneSpawner`)))

(fn `RandomizeLane`
  (params (FirstLane :type Boolean))
  (bind _returnvalue (`KismetMathLibrary.RandomIntegerInRange` 0 3))
  (if FirstLane
    (`KismetSystemLibrary.PrintString` "spawning first lane" true true (struct :`G` 0.66 :`B` 1.0 :`A` 1.0) 10.0)
    (for _index (range 3)
      (`StaticMeshComponent.SetStaticMesh` (select `int` _index :`0` (`self.lane2`) :`1` (`self.lane3`) :`2` (`self.lane1`)) "/Game/blender_export/field_type1.field_type1")
      (set `self.FieldType1` false))
    (else
      (bind _output_get (set `self.TempLaneSelectorInt` _returnvalue))
      ;[0.5161 1 0.5103] Used for alternating the field lane colors
      (for _index_2 (range 3)
        (if (== _returnvalue 0)
          (if (`self.FieldType1`)
            (for _index_3 (range 3)
              (`StaticMeshComponent.SetStaticMesh` (select `int` _index_3 :`0` (`self.lane2`) :`1` (`self.lane3`) :`2` (`self.lane1`)) "/Game/blender_export/field_type2.field_type2")
              (set `self.FieldType1` false)
              (`KismetSystemLibrary.PrintString` "field_type2")
              (`KismetSystemLibrary.PrintString` " spawned"))
            (else
              (bind _returnvalue_2 (select `int` _output_get :`0` "/Game/blender_export/field_type1.field_type1" :`1` "/Game/blender_export/FinalRiver.FinalRiver" :`2` "/Game/blender_export/road_type2.road_type2" :`3` "/Game/blender_export/TheFinalTrainTrack.TheFinalTrainTrack" :!type "StaticMesh Object Reference"))
              (`StaticMeshComponent.SetStaticMesh` (select `int` _index_2 :`0` (`self.lane2`) :`1` (`self.lane3`) :`2` (`self.lane1`)) _returnvalue_2 :!label _label)
              (`KismetSystemLibrary.PrintString` (`KismetSystemLibrary.GetDisplayName` _returnvalue_2))
              (`KismetSystemLibrary.PrintString` " spawned")))
          (else
            (goto _label)))))))

(fn `UserConstructionScript`)