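; Lane spawner actor that builds the opening run of randomized lanes at BeginPlay.
; SpawnInitialLane loops to place the first lane just below the player, then chains each next one at the newest lane's SpawnPoint.
; SpawnLane creates a BP_Lane, gives it a reference to the spawner and calls RandomizeLane on it.
; Older branches spawning separate road, river, train and field lane classes remain but never run.
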(event `self.ReceiveBeginPlay`
  (`self.SpawnInitialLane`))

(fn `Spawn Lane`
  (params (SpawnLocation :type "Vector Structure") (FirstLane :type Boolean))
  (bind _returnvalue (`|SpawnActorFromClass` "/Game/Blueprint/BP_Lane.BP_Lane_C" (`KismetMathLibrary.MakeTransform` SpawnLocation) "Undefined" "OverrideRootScale" null null))
  (bind _output_get (set `self.NewestLane` _returnvalue))
  (set `/Game/Blueprint/BP_Lane.MyLaneSpawner` self _output_get)
  (`/Game/Blueprint/BP_Lane.RandomizeLane` _output_get))

(fn `SpawnInitialLane`
  (for _index (range 6)
    (`KismetSystemLibrary.PrintText` (`KismetTextLibrary.Conv_IntToText` _index))
    (`/Engine/EditorBlueprintResources/StandardMacros.IsValid` null
      (:`Is Valid`
        (`self.SpawnLaneAtSpawnPoint`))
      (:`Is Not Valid`
        (`self.Spawn Lane` (- (`self.K2_GetActorLocation` (`GameplayStatics.GetPlayerCharacter` 0)) (0.0 0.0 20.0)) (`self.FirstLane`))))))

(fn `SpawnLaneAtSpawnPoint`
  (`self.Spawn Lane` (`SceneComponent.K2_GetComponentLocation` (`/Game/Blueprint/BP_Lane.SpawnPoint` (`self.NewestLane`)))))

(fn `UserConstructionScript`)