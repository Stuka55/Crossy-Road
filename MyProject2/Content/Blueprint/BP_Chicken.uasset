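; BP_Chicken is the player chicken character, which moves in short hops from the JumpForward and JumpRight axis inputs.
; Each hop uses LaunchCharacter, gated by Canmove and a DoOnce-plus-Delay cooldown.
; Forward-axis hops increment a tap counter on the WBP_HUD created at BeginPlay, which also shows coins.
; Positive JumpRight hops also play a timeline that updates the mesh rotation.
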(event `self.ReceiveBeginPlay`
  (bind _returnvalue (`|CreateWidget` "/Game/Blueprint/WBP_HUD.WBP_HUD_C"))
  (`UserWidget.AddToViewport` _returnvalue 0)
  (set `/Game/Blueprint/WBP_HUD.Chicken` self _returnvalue)
  (bind _output_get (set `self.MyHUD` _returnvalue))
  (`/Game/Blueprint/WBP_HUD.UpdateTapCounter` _output_get)
  (`/Game/Blueprint/WBP_HUD.UpdateCoinCounter` _output_get))

(event `InputAxis|JumpForward`
  (params (AxisValue :type "Float (single-precision)"))
  (if (and (> (`KismetMathLibrary.Abs` AxisValue) 0.3) (`self.canmove`))
    (`self.movementCooldown`)
    (`self.LaunchCharacter` (`KismetMathLibrary.MakeVector` (* AxisValue (`self.MovementSpace`)) 0.0 200.0) true true)
    (bind _result (`/Engine/EditorBlueprintResources/StandardMacros.IncrementInt` (`self.TapCounter`))
      (:`  `
        (set `self.TapCounter` _result)
        (`/Game/Blueprint/WBP_HUD.UpdateTapCounter` (`self.MyHUD`))))))

(event `InputAxis|JumpRight`
  (params (AxisValue :type "Float (single-precision)"))
  (bind _staticmesh (`self.StaticMesh`))
  (if (and (> (`KismetMathLibrary.Abs` AxisValue) 0.3) (`self.canmove`))
    (`self.movementCooldown`)
    (`self.LaunchCharacter` (`KismetMathLibrary.MakeVector` 0.0 (* AxisValue (`self.MovementSpace`)) 200.0) true true)
    (if (> AxisValue 0.3)
      (`Timeline|Timeline_0` :!via `PlayFromStart`
        (:`Update`
          (`SceneComponent.K2_SetWorldRotation` _staticmesh (`KismetMathLibrary.RLerp` (`SceneComponent.K2_GetComponentRotation` _staticmesh)) false false))))))

(event `movementCooldown`
  (`/Engine/EditorBlueprintResources/StandardMacros.DoOnce` false :!label _label
    (:`Completed`
      (set `self.canmove` false)
      (`KismetSystemLibrary.Delay` 0.45)
      (set `self.canmove` true)
      (goto _label :!via `Reset`))))

(fn `UserConstructionScript`)