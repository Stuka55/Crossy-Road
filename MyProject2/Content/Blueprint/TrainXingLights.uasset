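; Train crossing light actor that animates two point lights while a train is coming.
; Both lights start at zero intensity, and Tick plays a timeline whenever the Traincoming flag is true.
; The timeline's float and color tracks drive both lights' intensity and color, with a brightness multiplier applied only to PointLight1.
; The graph never sets the flag or stops the timeline.
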(event `self.ReceiveTick`
  (params (DeltaSeconds :type "Float (single-precision)"))
  (if (`self.Traincoming!`)
    (bind (_direction _lightbrighnessfloattrack _lightlinearcolortrack) (`Timeline|Timeline_0`)
      (:`Update`
        (`LightComponent.SetIntensity` (`self.PointLight1`) (* _lightbrighnessfloattrack (`self.BirghtnessMultiplier`)))
        (`LightComponent.SetIntensity` (`self.PointLight`) _lightbrighnessfloattrack)
        (`LightComponent.SetLightColor` (`self.PointLight1`) _lightlinearcolortrack true)
        (`LightComponent.SetLightColor` (`self.PointLight`) _lightlinearcolortrack true)))))

(event `self.ReceiveBeginPlay`
  (`LightComponent.SetIntensity` (`self.PointLight1`) 0.0)
  (`LightComponent.SetIntensity` (`self.PointLight`) 0.0))

(fn `UserConstructionScript`)