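; BP_car_type1 is a moving car obstacle that drives straight along its forward vector each tick, using a swept move.
; On BeginPlay, RandomCar picks one of eight jeep or sedan meshes; the police car option lies outside the random range and is never chosen.
; StopCarTriggerZone zeroes MoveSpeed while a BP_Chicken overlaps it and restores a hardcoded speed when the chicken leaves.
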(event `self.ReceiveBeginPlay`
  (`self.RandomCar`))

(event `self.ReceiveTick`
  (params (DeltaSeconds :type "Float (single-precision)"))
  (bind _output_get (set `self.Location` (`self.K2_GetActorLocation`)))
  (`self.K2_SetActorLocation` (+ (* DeltaSeconds (`self.MoveSpeed`) (`self.GetActorForwardVector`)) _output_get) true))

(event `self.StopCarTriggerZone.OnComponentBeginOverlap`
  (params (OverlappedComponent :type "PrimitiveComponent Object Reference") (OtherActor :type "Actor Object Reference") (OtherComp :type "PrimitiveComponent Object Reference") (OtherBodyIndex :type Integer) (bFromSweep :type Boolean) (SweepResult :type "HitResult Structure (by ref)"))
  (cast `/Game/Blueprint/BP_Chicken` OtherActor)
  (set `self.MoveSpeed` 0.0))

(event `self.StopCarTriggerZone.OnComponentEndOverlap`
  (params (OverlappedComponent :type "PrimitiveComponent Object Reference") (OtherActor :type "Actor Object Reference") (OtherComp :type "PrimitiveComponent Object Reference") (OtherBodyIndex :type Integer))
  (cast `/Game/Blueprint/BP_Chicken` OtherActor)
  (set `self.MoveSpeed` 500.0))

(fn `RandomCar`
  (`StaticMeshComponent.SetStaticMesh` (`self.StaticMesh`) (select `int` (`KismetMathLibrary.RandomIntegerInRange` 0 7) :`0` "/Game/blender_export/car_jeep_type1.car_jeep_type1" :`1` "/Game/blender_export/car_jeep_type2.car_jeep_type2" :`2` "/Game/blender_export/car_jeep_type3.car_jeep_type3" :`3` "/Game/blender_export/car_jeep_type4.car_jeep_type4" :`4` "/Game/blender_export/car_sedan_type1.car_sedan_type1" :`5` "/Game/blender_export/car_sedan_type2.car_sedan_type2" :`6` "/Game/blender_export/car_sedan_type3.car_sedan_type3" :`7` "/Game/blender_export/car_sedan_type4.car_sedan_type4" :`8` "/Game/blender_export/police_car_type1.police_car_type1" :!type "StaticMesh Object Reference")))

(fn `UserConstructionScript`)