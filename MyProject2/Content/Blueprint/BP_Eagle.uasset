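; Eagle actor Blueprint for a predator that dives in on the player's chicken, still partly stubbed.
; BeginPlay stores the player pawn's location and an offset point along X as variables, without moving the eagle to it.
; While GoingForTheKill is true, Tick shifts the actor by a fixed per-frame step along negative X and slightly downward, unscaled by delta time.
; SwoopToKill is empty, and nothing here sets the flag.
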(event `self.ReceiveTick`
  (params (DeltaSeconds :type "Float (single-precision)"))
  (if (`self.goingForTheKill?`)
    (`self.K2_SetActorLocation` (- (`self.K2_GetActorLocation`) (20.0 0.0 2.0)))))

(event `self.ReceiveBeginPlay`
  (bind _returnvalue (`self.K2_GetActorLocation` (`GameplayStatics.GetPlayerPawn` 0)))
  (set `self.ChickenLocation` _returnvalue)
  (set `self.EagleLocation` (+ _returnvalue (1000.0 0.0 0.0))))

(fn `Swoop to Kill`)

(fn `UserConstructionScript`)