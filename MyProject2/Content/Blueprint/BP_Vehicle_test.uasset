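; A test traffic vehicle that drives in a straight line and reacts to chickens in its path.
; On BeginPlay it picks a random car or truck mesh, then each tick moves along its right vector with a swept location update.
; Trigger overlaps with BP_Chicken play a horn or call the chicken's run-over or side-hit handler.
; Each reaction is gated by its own DoOnce with no reset, so it fires once per vehicle.
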(event `self.ReceiveBeginPlay`
  (`self.RandomVehicle`))

(event `self.ReceiveTick`
  (params (DeltaSeconds :type "Float (single-precision)"))
  (bind _output_get (set `self.Location` (`self.K2_GetActorLocation`)))
  (`self.K2_SetActorLocation` (+ (* DeltaSeconds (`self.Move Speed`) (`self.GetActorRightVector`)) _output_get) true))

(event `self.HonkAtChickenTrigger.OnComponentBeginOverlap`
  (params (OverlappedComponent :type "PrimitiveComponent Object Reference") (OtherActor :type "Actor Object Reference") (OtherComp :type "PrimitiveComponent Object Reference") (OtherBodyIndex :type Integer) (bFromSweep :type Boolean) (SweepResult :type "HitResult Structure (by ref)"))
  (cast `/Game/Blueprint/BP_Chicken` OtherActor)
  (`self.HonkDelay`))

(event `HonkDelay`
  (`/Engine/EditorBlueprintResources/StandardMacros.DoOnce` false
    (:`Completed`
      (`GameplayStatics.PlaySoundAtLocation` "/Game/audio/car-horn2_Cue.car-horn2_Cue" (`self.K2_GetActorLocation`) (struct) 1.0 1.0 0.0 null null null null))))

(event `self.RunOverChickenTriggerFront.OnComponentBeginOverlap`
  (params (OverlappedComponent :type "PrimitiveComponent Object Reference") (OtherActor :type "Actor Object Reference") (OtherComp :type "PrimitiveComponent Object Reference") (OtherBodyIndex :type Integer) (bFromSweep :type Boolean) (SweepResult :type "HitResult Structure (by ref)"))
  (bind _asbp_chicken (cast `/Game/Blueprint/BP_Chicken` OtherActor))
  (`/Engine/EditorBlueprintResources/StandardMacros.DoOnce` false
    (:`Completed`
      (`/Game/Blueprint/BP_Chicken.RanOverByCar` _asbp_chicken))))

(event `self.RunOverChickenTriggerSide.OnComponentBeginOverlap`
  (params (OverlappedComponent :type "PrimitiveComponent Object Reference") (OtherActor :type "Actor Object Reference") (OtherComp :type "PrimitiveComponent Object Reference") (OtherBodyIndex :type Integer) (bFromSweep :type Boolean) (SweepResult :type "HitResult Structure (by ref)"))
  (bind _asbp_chicken (cast `/Game/Blueprint/BP_Chicken` OtherActor))
  (`/Engine/EditorBlueprintResources/StandardMacros.DoOnce` false
    (:`Completed`
      (`/Game/Blueprint/BP_Chicken.HitSideOfCar` _asbp_chicken))))

(fn `RandomVehicle`
  (`StaticMeshComponent.SetStaticMesh` (`self.Vehicle`) (select `int` (`KismetMathLibrary.RandomIntegerInRange` 0 16) :`0` "/Game/blender_export/Pickup_Truck_Type1.Pickup_Truck_Type1" :`1` "/Game/blender_export/Pickup_Truck_Type2.Pickup_Truck_Type2" :`2` "/Game/blender_export/Pickup_Truck_Type3.Pickup_Truck_Type3" :`3` "/Game/blender_export/car_jeep_type1.car_jeep_type1" :`4` "/Game/blender_export/car_jeep_type2.car_jeep_type2" :`5` "/Game/blender_export/car_jeep_type3.car_jeep_type3" :`6` "/Game/blender_export/car_jeep_type4.car_jeep_type4" :`7` "/Game/blender_export/car_sedan_type1.car_sedan_type1" :`8` "/Game/blender_export/car_sedan_type2.car_sedan_type2" :`9` "/Game/blender_export/car_sedan_type3.car_sedan_type3" :`10` "/Game/blender_export/car_sedan_type4.car_sedan_type4" :`11` "/Game/blender_export/Car_type_5.Car_type_5" :`12` "/Game/blender_export/fireTruck.fireTruck" :`13` "/Game/blender_export/truck_type1.truck_type1" :`14` "/Game/blender_export/truck_type2.truck_type2" :`15` "/Game/blender_export/truck_type3.truck_type3" :`16` "/Game/blender_export/truck_type4.truck_type4" :!type "StaticMesh Object Reference")))

(fn `UserConstructionScript`)