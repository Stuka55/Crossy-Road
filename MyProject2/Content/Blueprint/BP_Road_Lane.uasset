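; Road lane actor for a chicken crossing game that spawns traffic and triggers creation of further lanes.
; On BeginPlay it picks one end as the car origin and starts a looping timer, with a 50% spawn chance per tick.
; The first chicken overlap on LaneSpawnTrigger calls LaneSpawner, and two destroy zones remove BP_car_type1 actors.
; Random lane-count logic is unwired, and RandomLane is empty.
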(event `self.ReceiveBeginPlay`
  (bind _output_get (set `self.StartLocation` (`SceneComponent.K2_GetComponentLocation` (`self.Start`))))
  (bind _output_get_2 (set `self.EndLocation` (`SceneComponent.K2_GetComponentLocation` (`self.End`))))
  (set `self.StartingCarLocation` (`KismetMathLibrary.RandomBool`))
  (`KismetSystemLibrary.K2_SetTimerDelegate` (delegate `SpawnVehicle`) (`KismetMathLibrary.RandomFloatInRange` 2.0 3.0) true))

(event `SpawnVehicle`
  (if (`KismetMathLibrary.RandomBool`)
    (if (`self.StartingCarLocation`)
      (`|SpawnActorFromClass` "/Game/Blueprint/VehicleSpawner.VehicleSpawner_C" (`KismetMathLibrary.MakeTransform` (stale `self.ReceiveBeginPlay` _output_get) (struct)) "Undefined" "OverrideRootScale" null null)
      (else
        (`|SpawnActorFromClass` "/Game/Blueprint/VehicleSpawner.VehicleSpawner_C" (`KismetMathLibrary.MakeTransform` (stale `self.ReceiveBeginPlay` _output_get_2) (struct)) "Undefined" "OverrideRootScale" null null)))))

(event `self.LaneSpawnTrigger.OnComponentBeginOverlap`
  (params (OverlappedComponent :type "PrimitiveComponent Object Reference") (OtherActor :type "Actor Object Reference") (OtherComp :type "PrimitiveComponent Object Reference") (OtherBodyIndex :type Integer) (bFromSweep :type Boolean) (SweepResult :type "HitResult Structure (by ref)"))
  (if (not (`self.Spawn ALane Yet?`))
    (cast `/Game/Blueprint/BP_Chicken` OtherActor)
    (`/Game/Blueprint/BP_LaneSpawner.SpawnLaneAtSpawnPoint` (`self.LaneSpawner`))
    (set `self.Spawn ALane Yet?` true)))

(event `self.DestroyCarZone.OnComponentBeginOverlap`
  (params (OverlappedComponent :type "PrimitiveComponent Object Reference") (OtherActor :type "Actor Object Reference") (OtherComp :type "PrimitiveComponent Object Reference") (OtherBodyIndex :type Integer) (bFromSweep :type Boolean) (SweepResult :type "HitResult Structure (by ref)"))
  (bind _asbp_car_type_1 (cast `/Game/Blueprint/BP_car_type1` OtherActor))
  (`self.K2_DestroyActor` _asbp_car_type_1))

(event `self.DestroyCarZone1.OnComponentBeginOverlap`
  (params (OverlappedComponent :type "PrimitiveComponent Object Reference") (OtherActor :type "Actor Object Reference") (OtherComp :type "PrimitiveComponent Object Reference") (OtherBodyIndex :type Integer) (bFromSweep :type Boolean) (SweepResult :type "HitResult Structure (by ref)"))
  (bind _asbp_car_type_1 (cast `/Game/Blueprint/BP_car_type1` OtherActor))
  (`self.K2_DestroyActor` _asbp_car_type_1))

(fn `RandomLane`)

(fn `UserConstructionScript`)