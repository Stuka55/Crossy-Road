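; BP_Pickup_truck is a traffic vehicle that drives along its forward vector at MoveSpeed every Tick, using a swept move.
; On BeginPlay, RandomPickup assigns a random mesh; five are wired, but the random range reaches only the three pickup types.
; Two trigger components halt it when a BP_Chicken or another pickup truck overlaps, and restore a fixed speed when that overlap ends, without checking for remaining blockers.
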(event `self.ReceiveBeginPlay`
  (`self.RandomPickup`))

(event `self.ReceiveTick`
  (params (DeltaSeconds :type "Float (single-precision)"))
  (bind _output_get (set `self.Location` (`self.K2_GetActorLocation`)))
  (`self.K2_SetActorLocation` (+ (* DeltaSeconds (`self.MoveSpeed`) (`self.GetActorForwardVector`)) _output_get) true))

(event `self.StopCaForChickenrTrigger.OnComponentBeginOverlap`
  (params (OverlappedComponent :type "PrimitiveComponent Object Reference") (OtherActor :type "Actor Object Reference") (OtherComp :type "PrimitiveComponent Object Reference") (OtherBodyIndex :type Integer) (bFromSweep :type Boolean) (SweepResult :type "HitResult Structure (by ref)"))
  (cast `/Game/Blueprint/BP_Chicken` OtherActor)
  (set `self.MoveSpeed` 0.0))

(event `self.StopCaForChickenrTrigger.OnComponentEndOverlap`
  (params (OverlappedComponent :type "PrimitiveComponent Object Reference") (OtherActor :type "Actor Object Reference") (OtherComp :type "PrimitiveComponent Object Reference") (OtherBodyIndex :type Integer))
  (cast `/Game/Blueprint/BP_Chicken` OtherActor)
  (set `self.MoveSpeed` 500.0))

(event `self.StopCaForCarTrigger1.OnComponentBeginOverlap`
  (params (OverlappedComponent :type "PrimitiveComponent Object Reference") (OtherActor :type "Actor Object Reference") (OtherComp :type "PrimitiveComponent Object Reference") (OtherBodyIndex :type Integer) (bFromSweep :type Boolean) (SweepResult :type "HitResult Structure (by ref)"))
  (bind _asbp_pickup_truck (cast `/Game/Blueprint/BP_Pickup_truck` OtherActor))
  (if (!= _asbp_pickup_truck self)
    (set `self.MoveSpeed` 0.0)))

(event `self.StopCaForCarTrigger1.OnComponentEndOverlap`
  (params (OverlappedComponent :type "PrimitiveComponent Object Reference") (OtherActor :type "Actor Object Reference") (OtherComp :type "PrimitiveComponent Object Reference") (OtherBodyIndex :type Integer))
  (cast `/Game/Blueprint/BP_Pickup_truck` OtherActor)
  (set `self.MoveSpeed` 500.0))

(fn `RandomPickup`
  (`StaticMeshComponent.SetStaticMesh` (`self.StaticMesh`) (select `int` (`KismetMathLibrary.RandomIntegerInRange` 0 2) :`0` "/Game/blender_export/Pickup_Truck_Type1.Pickup_Truck_Type1" :`1` "/Game/blender_export/Pickup_Truck_Type2.Pickup_Truck_Type2" :`2` "/Game/blender_export/Pickup_Truck_Type3.Pickup_Truck_Type3" :`3` "/Game/blender_export/Car_type_4.Car_type_4" :`4` "/Game/blender_export/Car_type_5.Car_type_5" :!type "StaticMesh Object Reference")))

(fn `UserConstructionScript`)