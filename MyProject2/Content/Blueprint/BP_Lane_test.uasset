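; Test lane Blueprint for a Crossy Road-style chicken game, randomized as field, river, road or train track.
; RandomizeLane sets LaneID, swaps five lane meshes and calls per-type spawn events, of which only log spawning is implemented.
; River logs spawn on a looping timer by coin flip, from either end, chosen once.
; BP_Chicken overlaps trigger the next lane spawn and HUD counter increment, or drowning on river lanes.
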(event `SpawnRailRoadTracksNLights`)

(event `SpawnCars`)

(event `SpawnRocksNTrees`)

(event `spawnLog`
  (bind _output_get (set `self.StartLocation` (`SceneComponent.K2_GetComponentLocation` (`self.Start`))))
  (bind _output_get_2 (set `self.EndLocation` (`SceneComponent.K2_GetComponentLocation` (`self.End`))))
  (set `self.StartingLogLocation` (`KismetMathLibrary.RandomBool`))
  (`KismetSystemLibrary.K2_SetTimerDelegate` (delegate `SpawnLogs`) (`KismetMathLibrary.RandomFloatInRange` 7.0 10.0) true))

(event `SpawnLogs`
  (if (`KismetMathLibrary.RandomBool`)
    (if (`self.StartingLogLocation`)
      (`|SpawnActorFromClass` "/Game/Blueprint/BP_LogSpawner.BP_LogSpawner_C" (`KismetMathLibrary.MakeTransform` (stale `spawnLog` _output_get)) "Undefined" "OverrideRootScale" null null)
      (else
        (`|SpawnActorFromClass` "/Game/Blueprint/BP_LogSpawner.BP_LogSpawner_C" (`KismetMathLibrary.MakeTransform` (stale `spawnLog` _output_get_2)) "Undefined" "OverrideRootScale" null null)))))

(event `self.ReceiveBeginPlay`)

(event `self.TriggerZone.OnComponentBeginOverlap`
  (params (OverlappedComponent :type "PrimitiveComponent Object Reference") (OtherActor :type "Actor Object Reference") (OtherComp :type "PrimitiveComponent Object Reference") (OtherBodyIndex :type Integer) (bFromSweep :type Boolean) (SweepResult :type "HitResult Structure (by ref)"))
  (bind _asbp_chicken (cast `/Game/Blueprint/BP_Chicken` OtherActor))
  (`/Game/Blueprint/BP_LaneSpawner.Spawn Lane at Spawn Point` (`self.MyLaneSpawner`) false)
  (`ActorComponent.K2_DestroyComponent` (`self.TriggerZone`))
  (bind _result (`/Engine/EditorBlueprintResources/StandardMacros.IncrementInt` (`/Game/Blueprint/BP_Chicken.TapCounter` _asbp_chicken))
    (:`  `
      (set `/Game/Blueprint/BP_Chicken.TapCounter` _result _asbp_chicken)
      (`/Game/Blueprint/WBP_HUD.UpdateTapCounter` (`/Game/Blueprint/BP_Chicken.MyHUD` _asbp_chicken)))))

(event `self.WaterTrigger.OnComponentBeginOverlap`
  (params (OverlappedComponent :type "PrimitiveComponent Object Reference") (OtherActor :type "Actor Object Reference") (OtherComp :type "PrimitiveComponent Object Reference") (OtherBodyIndex :type Integer) (bFromSweep :type Boolean) (SweepResult :type "HitResult Structure (by ref)"))
  (bind _asbp_chicken (cast `/Game/Blueprint/BP_Chicken` OtherActor))
  (`/Engine/EditorBlueprintResources/StandardMacros.DoOnce` false
    (:`Completed`
      (if (== 1 (`self.LaneID`))
        (`/Game/Blueprint/BP_Chicken.FallInWater` _asbp_chicken)))))

(fn `RandomizeLane`
  (params (FirstLane :type Boolean))
  (if FirstLane
    (for _index (range 5)
      (`StaticMeshComponent.SetStaticMesh` (select `int` _index :`0` (`self.lane2`) :`1` (`self.lane3`) :`2` (`self.lane1`) :`3` (`self.lane4`) :`4` (`self.lane5`)) "/Game/blender_export/field_type1.field_type1")
      (set `self.FieldType1` false)
      (set `self.LaneID` 0)
      (switch `int` (`self.LaneID`) :!label _label
        (:`0`
          (`self.SpawnRocksNTrees`))
        (:`1`
          (`self.spawnLog`))
        (:`2`
          (`self.SpawnCars`))
        (:`3`
          (`self.SpawnRailRoadTracksNLights`))))
    (else
      (bind _output_get (set `self.TempLaneSelectorInt` (`KismetMathLibrary.RandomIntegerInRange` 0 3)))
      (bind _output_get_2 (set `self.LaneID` _output_get))
      (`KismetSystemLibrary.PrintString` (`KismetStringLibrary.Conv_IntToString` _output_get_2) true true (struct :`G` 0.66 :`B` 1.0 :`A` 1.0) 10.0)
      ;[0.5161 1 0.5103] Used for alternating the field lane colors
      (for _index_2 (range 5)
        (if (== _output_get 0)
          (if (`self.FieldType1`)
            (for _index_3 (range 3)
              (`StaticMeshComponent.SetStaticMesh` (select `int` _index_3 :`0` (`self.lane2`) :`1` (`self.lane3`) :`2` (`self.lane1`)) "/Game/blender_export/field_type2.field_type2")
              (set `self.FieldType1` false)
              (goto _label))
            (else
              (`StaticMeshComponent.SetStaticMesh` (select `int` _index_2 :`0` (`self.lane2`) :`1` (`self.lane3`) :`2` (`self.lane1`) :`3` (`self.lane4`) :`4` (`self.lane5`)) (select `int` _output_get :`0` "/Game/blender_export/field_type1.field_type1" :`1` "/Game/blender_export/FinalRiver.FinalRiver" :`2` "/Game/blender_export/road_type2.road_type2" :`3` "/Game/blender_export/TheFinalTrainTrack.TheFinalTrainTrack" :!type "StaticMesh Object Reference") :!label _label_2)))
          (else
            (goto _label_2)))))))

(fn `UserConstructionScript`)