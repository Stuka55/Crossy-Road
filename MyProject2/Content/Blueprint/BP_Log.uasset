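; BP_Log is a moving log actor that takes on one of three random looks.
; On BeginPlay, RandomLog picks a random static mesh from the three log type variables and assigns it to the Log component.
; Every Tick it moves along its right vector at MoveSpeed, scaled by delta time, using a swept SetActorLocation.
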(event `self.ReceiveBeginPlay`
  (`self.RandomLog`))

(event `self.ReceiveTick`
  (params (DeltaSeconds :type "Float (single-precision)"))
  (bind _output_get (set `self.Location` (`self.K2_GetActorLocation`)))
  (`self.K2_SetActorLocation` (+ (* DeltaSeconds (`self.MoveSpeed`) (`self.GetActorRightVector`)) _output_get) true))

(fn `RandomLog`
  (`StaticMeshComponent.SetStaticMesh` (`self.Log`) (select `int` (`KismetMathLibrary.RandomIntegerInRange` 0 2) :`0` "/Game/blender_export/LogType1.LogType1" :`1` "/Game/blender_export/LogType2.LogType2" :`2` "/Game/blender_export/LogType3.LogType3" :!type "StaticMesh Object Reference")))

(fn `UserConstructionScript`)