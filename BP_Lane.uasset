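; BP_Lane is one strip of a Crossy Road-style chicken game, randomized as field, river, road or railway.
; RandomizeLane sets LaneID and meshes, then spawns trees and rocks or coins, or starts looping timers for logs, cars, or trains with crossing lights.
; Chicken overlap advances score, resets the eagle countdown, requests another lane and schedules self-destruction.
; Edge zones destroy vehicles, trains and logs; water and kill zones trigger FallInWater.
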(event `SpawnBunchOfTrees`
  (bind (_startlocation_x _startlocation_y _startlocation_z) (`KismetMathLibrary.BreakVector` (`self.StartLocation`)))
  (set `self.StartLocation` (`SceneComponent.K2_GetComponentLocation` (`self.end`)))
  (set `self.EndLocation` (`SceneComponent.K2_GetComponentLocation` (`self.start`)))
  (for _index (range (+ (`KismetMathLibrary.FTrunc` (/ (`KismetMathLibrary.Vector_Distance` (`self.StartLocation`) (`self.EndLocation`)) 40.0)) 1))
    (bind _returnvalue (`|SpawnActorFromClass` "/Game/Blueprint/BP_Tree_rock_spawner.BP_Tree_rock_spawner_C" (`KismetMathLibrary.MakeTransform` (`KismetMathLibrary.MakeVector` _startlocation_x (+ (.y (`self.StartLocation`)) (* _index (* (`KismetMathLibrary.RandomFloat`) 50.0))) _startlocation_z)) "Undefined" "OverrideRootScale" null null))
    (`KismetArrayLibrary.Array_Add` (`self.MyTreeAndRockSpawnerArray`) _returnvalue)))

(event `CountDown to delete`
  (`KismetSystemLibrary.Delay` 30.0)
  (`self.K2_DestroyActor`)
  (`self.K2_DestroyActor` (`self.MyTreeAndRockSpawnerArray`))
  (`self.K2_DestroyActor`))

(event `CoinSpawner`
  (params (ThisLane :type "/BP_Lane Object Reference"))
  (bind (_startlocation_x _startlocation_y _startlocation_z) (`KismetMathLibrary.BreakVector` (`self.StartLocation`)))
  (bind _output_get (set `self.StartLocation` (`SceneComponent.K2_GetComponentLocation` (`self.end`))))
  (bind _output_get_2 (set `self.EndLocation` (`SceneComponent.K2_GetComponentLocation` (`self.start`))))
  (for _index (range (+ (`KismetMathLibrary.FTrunc` (/ (`KismetMathLibrary.Vector_Distance` _output_get _output_get_2) 85.0)) 1))
    (if (> (`KismetMathLibrary.RandomFloat`) 0.995)
      (`|SpawnActorFromClass` "/Game/Blueprint/BP_Coin.BP_Coin_C" (`KismetMathLibrary.MakeTransform` (`KismetMathLibrary.MakeVector` _startlocation_x (+ (.y (`self.StartLocation`)) (* _index 90.0)) (+ _startlocation_z 17.0))) "Undefined" "OverrideRootScale" null null))))

(event `SpawnRailRoadTracksNLights`
  (params (ThisLane :type "/BP_Lane Object Reference"))
  (bind _output_get (set `self.StartLocation` (`SceneComponent.K2_GetComponentLocation` (`self.Start`))))
  (bind _output_get_2 (set `self.EndLocation` (`SceneComponent.K2_GetComponentLocation` (`self.End`))))
  (set `self.StartingCarLocation` (`KismetMathLibrary.RandomBool`))
  (`KismetSystemLibrary.K2_SetTimerDelegate` (delegate `CustomEvent`) (`KismetMathLibrary.RandomFloatInRange` 5.0 10.0) true))

(event `CustomEvent`
  (if (`KismetMathLibrary.RandomBool`)
    (if (`self.StartingCarLocation`)
      (for _array_element (`self.MyTrainXIngLightBP`)
        (set `/Game/Blueprint/TrainXingLights.Traincoming!` true _array_element)
        (`GameplayStatics.PlaySoundAtLocation` "/Game/audio/train-crossing_Cue.train-crossing_Cue" (`self.K2_GetActorLocation` _array_element) (struct) 1.0 1.0 0.0 null null null null))
      (`KismetSystemLibrary.Delay` 2.5)
      (bind _returnvalue (`|SpawnActorFromClass` "/Game/Blueprint/BP_Train.BP_Train_C" (`KismetMathLibrary.MakeTransform` (stale `SpawnRailRoadTracksNLights` _output_get) (struct :`Yaw` 90.0) (2.0 2.0 2.0)) "Undefined" "OverrideRootScale" null null))
      (`GameplayStatics.PlaySoundAtLocation` "/Game/audio/train-whistle-WAV.train-whistle-WAV" (`self.K2_GetActorLocation` _returnvalue) (struct) 1.0 1.0 0.0 null null null null)
      (else
        (for _array_element_2 (`self.MyTrainXIngLightBP`)
          (set `/Game/Blueprint/TrainXingLights.Traincoming!` true _array_element_2)
          (`GameplayStatics.PlaySoundAtLocation` "/Game/audio/train-crossing_Cue.train-crossing_Cue" (`self.K2_GetActorLocation` _array_element_2) (struct) 1.0 1.0 0.0 null null null null))
        (`KismetSystemLibrary.Delay` 2.5)
        (`|SpawnActorFromClass` "/Game/Blueprint/BP_Train.BP_Train_C" (`KismetMathLibrary.MakeTransform` (stale `SpawnRailRoadTracksNLights` _output_get_2) (struct :`Yaw` -90.0) (2.0 2.0 2.0)) "Undefined" "OverrideRootScale" null null)))))

(event `SpawnRocksNTrees`
  (params (ThisLane :type "/BP_Lane Object Reference"))
  (bind (_startlocation_x _startlocation_y _startlocation_z) (`KismetMathLibrary.BreakVector` (`self.StartLocation`)))
  (set `self.StartLocation` (`SceneComponent.K2_GetComponentLocation` (`self.end`)))
  (set `self.EndLocation` (`SceneComponent.K2_GetComponentLocation` (`self.start`)))
  (for _index (range (+ (`KismetMathLibrary.FTrunc` (/ (`KismetMathLibrary.Vector_Distance` (`self.StartLocation`) (`self.EndLocation`)) 85.0)) 1))
    (if (> (`KismetMathLibrary.RandomFloat`) 0.9)
      (if (not true)
        (`self.CoinSpawner` null))
      (elif (> (`KismetMathLibrary.RandomFloat`) 0.8)
        (bind _returnvalue (`|SpawnActorFromClass` "/Game/Blueprint/BP_Tree_rock_spawner.BP_Tree_rock_spawner_C" (`KismetMathLibrary.MakeTransform` (`KismetMathLibrary.MakeVector` _startlocation_x (+ (.y (`self.StartLocation`)) (* _index (* (`KismetMathLibrary.RandomFloat`) 10000.0))) _startlocation_z)) "Undefined" "OverrideRootScale" null null))
        (bind _returnvalue_2 (`KismetArrayLibrary.Array_Add` (`self.MyTreeAndRockSpawnerArray`) _returnvalue))))))

(event `SpawnCars`
  (bind _output_get (set `self.StartLocation` (`SceneComponent.K2_GetComponentLocation` (`self.Start`))))
  (bind _output_get_2 (set `self.EndLocation` (`SceneComponent.K2_GetComponentLocation` (`self.End`))))
  (set `self.StartingCarLocation` (`KismetMathLibrary.RandomBool`))
  (`KismetSystemLibrary.K2_SetTimerDelegate` (delegate `SpawnCARR`) (`KismetMathLibrary.RandomFloatInRange` 2.0 3.0) true))

(event `SpawnCARR`
  (if (`KismetMathLibrary.RandomBool`)
    (if (`self.StartingCarLocation`)
      (`|SpawnActorFromClass` "/Game/Blueprint/BP_Vehicle.BP_Vehicle_C" (`KismetMathLibrary.MakeTransform` (stale `SpawnCars` _output_get) (struct :`Yaw` 90.0)) "Undefined" "OverrideRootScale" null null)
      (else
        (`|SpawnActorFromClass` "/Game/Blueprint/BP_Vehicle.BP_Vehicle_C" (`KismetMathLibrary.MakeTransform` (stale `SpawnCars` _output_get_2) (struct :`Yaw` -90.0)) "Undefined" "OverrideRootScale" null null)))))

(event `spawnLog`
  (bind _output_get (set `self.StartLocation` (`SceneComponent.K2_GetComponentLocation` (`self.Start`))))
  (bind _output_get_2 (set `self.EndLocation` (`SceneComponent.K2_GetComponentLocation` (`self.End`))))
  (set `self.StartingLogLocation` (`KismetMathLibrary.RandomBool`))
  (`KismetSystemLibrary.K2_SetTimerDelegate` (delegate `SpawnLogs`) (`KismetMathLibrary.RandomFloatInRange` 1.0 2.5) true))

(event `SpawnLogs`
  (if (>= (`KismetMathLibrary.RandomFloat`) 0.3)
    (if (`self.StartingLogLocation`)
      (`|SpawnActorFromClass` "/Game/Blueprint/BP_Log.BP_Log_C" (`KismetMathLibrary.MakeTransform` (stale `spawnLog` _output_get) (struct :`Yaw` -90.0)) "Undefined" "OverrideRootScale" null null)
      (else
        (`|SpawnActorFromClass` "/Game/Blueprint/BP_Log.BP_Log_C" (`KismetMathLibrary.MakeTransform` (stale `spawnLog` _output_get_2) (struct :`Yaw` 90.0)) "Undefined" "OverrideRootScale" null null)))))

(event `self.ReceiveBeginPlay`)

(event `self.TriggerZone.OnComponentBeginOverlap`
  (params (OverlappedComponent :type "PrimitiveComponent Object Reference") (OtherActor :type "Actor Object Reference") (OtherComp :type "PrimitiveComponent Object Reference") (OtherBodyIndex :type Integer) (bFromSweep :type Boolean) (SweepResult :type "HitResult Structure (by ref)"))
  (bind _asbp_chicken (cast `/Game/Blueprint/BP_Chicken` OtherActor))
  (set `/Game/Blueprint/BP_Chicken.CountDownTillEagleDeath` 10.0 _asbp_chicken)
  (`/Game/Blueprint/BP_LaneSpawner.Spawn Lane at Spawn Point` (`self.MyLaneSpawner`) false)
  (`ActorComponent.K2_DestroyComponent` (`self.TriggerZone`))
  (bind _result (`/Engine/EditorBlueprintResources/StandardMacros.IncrementInt` (`/Game/Blueprint/BP_Chicken.TapCounter` _asbp_chicken))
    (:`  `
      (set `/Game/Blueprint/BP_Chicken.TapCounter` _result _asbp_chicken)
      (`/Game/Blueprint/WBP_HUD.UpdateTapCounter` (`/Game/Blueprint/BP_Chicken.MyHUD` _asbp_chicken))
      (`self.CountDown to delete`))))

(event `self.DestroyCarZone1.OnComponentBeginOverlap`
  (params (OverlappedComponent :type "PrimitiveComponent Object Reference") (OtherActor :type "Actor Object Reference") (OtherComp :type "PrimitiveComponent Object Reference") (OtherBodyIndex :type Integer) (bFromSweep :type Boolean) (SweepResult :type "HitResult Structure (by ref)"))
  (bind _asbp_vehicle (cast `/Game/Blueprint/BP_Vehicle` OtherActor))
  (`self.K2_DestroyActor` _asbp_vehicle))

(event `self.DestroyCarZone.OnComponentBeginOverlap`
  (params (OverlappedComponent :type "PrimitiveComponent Object Reference") (OtherActor :type "Actor Object Reference") (OtherComp :type "PrimitiveComponent Object Reference") (OtherBodyIndex :type Integer) (bFromSweep :type Boolean) (SweepResult :type "HitResult Structure (by ref)"))
  (bind _asbp_vehicle (cast `/Game/Blueprint/BP_Vehicle` OtherActor))
  (`self.K2_DestroyActor` _asbp_vehicle))

(event `self.WaterTrigger.OnComponentBeginOverlap`
  (params (OverlappedComponent :type "PrimitiveComponent Object Reference") (OtherActor :type "Actor Object Reference") (OtherComp :type "PrimitiveComponent Object Reference") (OtherBodyIndex :type Integer) (bFromSweep :type Boolean) (SweepResult :type "HitResult Structure (by ref)"))
  (bind _asbp_chicken (cast `/Game/Blueprint/BP_Chicken` OtherActor))
  (`/Engine/EditorBlueprintResources/StandardMacros.DoOnce` false
    (:`Completed`
      (if (== 1 (`self.LaneID`))
        (`/Game/Blueprint/BP_Chicken.FallInWater` _asbp_chicken)))))

(event `self.ChickenKillZone1.OnComponentBeginOverlap`
  (params (OverlappedComponent :type "PrimitiveComponent Object Reference") (OtherActor :type "Actor Object Reference") (OtherComp :type "PrimitiveComponent Object Reference") (OtherBodyIndex :type Integer) (bFromSweep :type Boolean) (SweepResult :type "HitResult Structure (by ref)"))
  (bind _asbp_chicken (cast `/Game/Blueprint/BP_Chicken` OtherActor))
  (`/Game/Blueprint/BP_Chicken.FallInWater` _asbp_chicken))

(event `self.ChickenKillZone2.OnComponentBeginOverlap`
  (params (OverlappedComponent :type "PrimitiveComponent Object Reference") (OtherActor :type "Actor Object Reference") (OtherComp :type "PrimitiveComponent Object Reference") (OtherBodyIndex :type Integer) (bFromSweep :type Boolean) (SweepResult :type "HitResult Structure (by ref)"))
  (bind _asbp_chicken (cast `/Game/Blueprint/BP_Chicken` OtherActor))
  (`/Game/Blueprint/BP_Chicken.FallInWater` _asbp_chicken))

(event `self.DestroyTrainZone1.OnComponentBeginOverlap`
  (params (OverlappedComponent :type "PrimitiveComponent Object Reference") (OtherActor :type "Actor Object Reference") (OtherComp :type "PrimitiveComponent Object Reference") (OtherBodyIndex :type Integer) (bFromSweep :type Boolean) (SweepResult :type "HitResult Structure (by ref)"))
  (bind _asbp_train (cast `/Game/Blueprint/BP_Train` OtherActor))
  (`self.K2_DestroyActor` _asbp_train))

(event `self.DestroyTrainZone2.OnComponentBeginOverlap`
  (params (OverlappedComponent :type "PrimitiveComponent Object Reference") (OtherActor :type "Actor Object Reference") (OtherComp :type "PrimitiveComponent Object Reference") (OtherBodyIndex :type Integer) (bFromSweep :type Boolean) (SweepResult :type "HitResult Structure (by ref)"))
  (bind _asbp_train (cast `/Game/Blueprint/BP_Train` OtherActor))
  (`self.K2_DestroyActor` _asbp_train))

(event `self.DestroyLogZone1.OnComponentBeginOverlap`
  (params (OverlappedComponent :type "PrimitiveComponent Object Reference") (OtherActor :type "Actor Object Reference") (OtherComp :type "PrimitiveComponent Object Reference") (OtherBodyIndex :type Integer) (bFromSweep :type Boolean) (SweepResult :type "HitResult Structure (by ref)"))
  (bind _asbp_log (cast `/Game/Blueprint/BP_Log` OtherActor))
  (`self.K2_DestroyActor` _asbp_log))

(event `self.DestroyLogZone2.OnComponentBeginOverlap`
  (params (OverlappedComponent :type "PrimitiveComponent Object Reference") (OtherActor :type "Actor Object Reference") (OtherComp :type "PrimitiveComponent Object Reference") (OtherBodyIndex :type Integer) (bFromSweep :type Boolean) (SweepResult :type "HitResult Structure (by ref)"))
  (bind _asbp_log (cast `/Game/Blueprint/BP_Log` OtherActor))
  (`self.K2_DestroyActor` _asbp_log))

(fn `RandomizeLane`
  (params (FirstLane :type Boolean) (`LaneMarker?` :type Boolean) (LastLaneWasFieldType1 :type Boolean) (InitialLane :type Boolean))
  (bind _mylanespawner (`self.MyLaneSpawner`))
  (if FirstLane
    (set `self.FirstLane` true)
    (for _index (range 5) :!label _label
      (`StaticMeshComponent.SetStaticMesh` (select `int` _index :`0` (`self.lane2`) :`1` (`self.lane3`) :`2` (`self.lane1`) :`3` (`self.lane4`) :`4` (`self.lane5`)) "/Game/blender_export/field_type1.field_type1")
      (set `self.LastLaneWasFieldType1` false)
      (set `self.LaneID` 0)
      (switch `int` (`self.LaneID`) :!label _label_2
        (:`0`
          (if (`self.FirstLane`)
            (`self.SpawnBunchOfTrees`)
            (set `self.FirstLane` false)
            (else
              (`self.SpawnRocksNTrees` self))))
        (:`1`
          (`self.spawnLog`))
        (:`2`
          (`self.SpawnCars` :!label _label_3)
          (`self.CoinSpawner` null :!label _label_4)
          (if (== 2 (`self.LaneID`))
            (`/Engine/EditorBlueprintResources/StandardMacros.DoOnce` false
              (:`Completed`
                (for _ (range (+ (`KismetMathLibrary.RandomIntegerInRange` 0 3) 1))
                  (`/Game/Blueprint/BP_LaneSpawner.SpawnRoadLanes` _mylanespawner)
                  (`self.SpawnCars` (`/Game/Blueprint/BP_LaneSpawner.NewestLane` _mylanespawner)))))))
        (:`3`
          (`self.SpawnRailRoadTracksNLights` null)
          (bind _output_get (set `self.TrainLight1` (`SceneComponent.K2_GetComponentLocation` (`self.TrainL1`))))
          (bind _output_get_2 (set `self.TrainLight3` (`SceneComponent.K2_GetComponentLocation` (`self.TrainL3`))))
          (bind _output_get_3 (set `self.TrainLight2` (`SceneComponent.K2_GetComponentLocation` (`self.TrainL2`))))
          (for _index_2 (range 4)
            (bind _returnvalue (`|SpawnActorFromClass` "/Game/Blueprint/TrainXingLights.TrainXingLights_C" (`KismetMathLibrary.MakeTransform` (- (select `int` _index_2 :`0` _output_get :`1` _output_get_2 :`2` _output_get_3) (0.0 0.0 200.0)) (struct :`Yaw` 90.0)) "Undefined" "OverrideRootScale" null null))
            (`KismetArrayLibrary.Array_Add` (`self.MyTrainXIngLightBP`) _returnvalue)
            (goto _label_4)))
        (:`4`
          (goto _label_3))))
    (elif InitialLane
      (goto _label)
      (else
        (if (> (`KismetMathLibrary.RandomIntegerInRange` 0 3) 1)
          (if (>= (`KismetMathLibrary.RandomFloat`) 0.25)
            (bind _output_get_4 (set `self.TempLaneSelectorInt` (`KismetMathLibrary.RandomIntegerInRange` 1 3)))
            (else
              (set `self.TempLaneSelectorInt` 0 :!label _label_5)))
          (else
            (goto _label_5)))
        (bind _output_get_5 (set `self.LaneID` _output_get_4))
        (if (== _output_get_5 2)
          (if `LaneMarker?`
            (set `self.LaneID` 4)
            (else
              (set `self.IsRoadWithoutMarker` true))))
        ;[0.5161 1 0.5103] Used for alternating the field lane colors
        (for _index_3 (range 5)
          (if (== _output_get_5 0)
            (set `self.LaneID` 0)
            (if (`self.LastLaneWasFieldType1`)
              (for _index_4 (range 5)
                (`StaticMeshComponent.SetStaticMesh` (select `int` _index_4 :`0` (`self.lane2`) :`1` (`self.lane3`) :`2` (`self.lane1`) :`3` (`self.lane4`) :`4` (`self.lane5`)) "/Game/blender_export/field_type2.field_type2")
                (set `self.LastLaneWasFieldType1` false)
                (goto _label_2))
              (else
                (set `self.LastLaneWasFieldType1` true)
                (`StaticMeshComponent.SetStaticMesh` (select `int` _index_3 :`0` (`self.lane2`) :`1` (`self.lane3`) :`2` (`self.lane1`) :`3` (`self.lane4`) :`4` (`self.lane5`)) (select `int` (`self.LaneID`) :`0` "/Game/blender_export/field_type1.field_type1" :`1` "/Game/blender_export/FinalRiver.FinalRiver" :`2` "/Game/blender_export/road_type2.road_type2" :`3` "/Game/blender_export/TheFinalTrainTrack.TheFinalTrainTrack" :`4` "/Game/blender_export/road_type1.road_type1" :!type "StaticMesh Object Reference") :!label _label_6)
                (goto _label_2)))
            (else
              (goto _label_6))))))))

(fn `setRoadMesh`
  (for _index (range 5)
    (bind _returnvalue (select `int` _index :`0` (`self.lane2`) :`1` (`self.lane3`) :`2` (`self.lane1`) :`3` (`self.lane4`) :`4` (`self.lane5`)))
    (`StaticMeshComponent.SetStaticMesh` _returnvalue "/Game/blender_export/road_type1.road_type1")
    (`SceneComponent.K2_AddLocalRotation` _returnvalue (struct :`Yaw` 180.0) false true)
    (`SceneComponent.K2_AddLocalOffset` _returnvalue (0.0 -20.0 0.0) false true)
    (set `self.LaneID` 4)
    (`self.SpawnCars`)))

(fn `UserConstructionScript`)