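; Spawner actor that builds the terrain as a chain of BP_Lane actors, each placed at the previous lane's SpawnPoint.
; On BeginPlay it places the first lane relative to the player, then extends the chain in batches, sized larger during initial setup.
; Each lane gets a back-reference to the spawner and randomizes itself using first, initial or road-marker context.
; SpawnRoadLanes instead appends a lane with a forced road mesh.
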(event `self.ReceiveBeginPlay`
  (`self.SpawnInitialLane`))

(fn `Spawn Lane`
  (params (SpawnLocation :type "Vector Structure") (FirstLane :type Boolean) (`LaneMarker?` :type Boolean) (`AreInitialLanes?` :type Boolean))
  (if FirstLane
    (bind _returnvalue (`|SpawnActorFromClass` "/Game/Blueprint/BP_Lane.BP_Lane_C" (`KismetMathLibrary.MakeTransform` SpawnLocation) "Undefined" "OverrideRootScale" null null :!label _label))
    (bind _output_get (set `self.NewestLane` _returnvalue))
    (set `/Game/Blueprint/BP_Lane.MyLaneSpawner` self _output_get)
    (`/Game/Blueprint/BP_Lane.RandomizeLane` _output_get FirstLane false false `AreInitialLanes?`)
    (if (`self.FirstLane`)
      (set `self.FirstLane` false))
    (elif `AreInitialLanes?`
      (goto _label)
      (elif `LaneMarker?`
        (bind _returnvalue_2 (`|SpawnActorFromClass` "/Game/Blueprint/BP_Lane.BP_Lane_C" (`KismetMathLibrary.MakeTransform` SpawnLocation) "Undefined" "OverrideRootScale" null null))
        (bind _output_get_2 (set `self.NewestLane` _returnvalue_2))
        (set `/Game/Blueprint/BP_Lane.MyLaneSpawner` self _output_get_2)
        (`/Game/Blueprint/BP_Lane.RandomizeLane` _output_get_2 false (`/Game/Blueprint/BP_Lane.IsRoadWithoutMarker` _output_get_2) false false)
        (else
          (bind _returnvalue_3 (`|SpawnActorFromClass` "/Game/Blueprint/BP_Lane.BP_Lane_C" (`KismetMathLibrary.MakeTransform` SpawnLocation) "Undefined" "OverrideRootScale" null null))
          (bind _output_get_3 (set `self.NewestLane` _returnvalue_3))
          (set `/Game/Blueprint/BP_Lane.MyLaneSpawner` self _output_get_3)
          (`/Game/Blueprint/BP_Lane.RandomizeLane` _output_get_3 false false false false))))))

(fn `Spawn Lane at Spawn Point`
  (params (`AreInitialLanes?` :type Boolean))
  (if `AreInitialLanes?`
    (for _ (range 4)
      (`self.Spawn Lane` (`SceneComponent.K2_GetComponentLocation` (`/Game/Blueprint/BP_Lane.SpawnPoint` (`self.NewestLane`))) false false `AreInitialLanes?` :!label _label))
    (set `self.AreInitialLanes?` false)
    (else
      (for _ (range 2)
        (goto _label)))))

(fn `SpawnInitialLane`
  ;[1 1 1] Used for changing the number of initial terrain spawned
  (for _index (range 6)
    (`KismetSystemLibrary.PrintString` "spawning init lane " true true (struct :`G` 0.66 :`B` 1.0 :`A` 1.0) 10.0)
    (`KismetSystemLibrary.PrintString` (`KismetStringLibrary.Conv_IntToString` _index) true true (struct :`G` 0.66 :`B` 1.0 :`A` 1.0) 10.0)
    (`/Engine/EditorBlueprintResources/StandardMacros.IsValid` (`self.NewestLane`)
      (:`Is Valid`
        (`self.Spawn Lane at Spawn Point` (`self.AreInitialLanes?`)))
      (:`Is Not Valid`
        (`self.Spawn Lane` (- (`self.K2_GetActorLocation` (`GameplayStatics.GetPlayerCharacter` 0)) (400.0 0.0 100.0)) (`self.FirstLane`))))))

(fn `SpawnRoadLanes`
  (bind _returnvalue (`|SpawnActorFromClass` "/Game/Blueprint/BP_Lane.BP_Lane_C" (`KismetMathLibrary.MakeTransform` (`SceneComponent.K2_GetComponentLocation` (`/Game/Blueprint/BP_Lane.SpawnPoint` (`self.NewestLane`)))) "Undefined" "OverrideRootScale" null null))
  (bind _output_get (set `self.NewestLane` _returnvalue))
  (set `/Game/Blueprint/BP_Lane.MyLaneSpawner` self _output_get)
  (`/Game/Blueprint/BP_Lane.setRoadMesh` _output_get))

(fn `UserConstructionScript`)